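; Runtime terrain generator actor that builds terrain from surface and height map images loaded from disk.
; On BeginPlay it shows a generation menu widget and enables mouse input.
; The menu's generate event loads both textures, reports invalid paths as red status text, or shows a progress bar and starts chunked terrain generation using the given height strength.
; A completion event hides the progress bar.
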(event Custom|On%20Genrate_Event
  (params (SurfaceMapPath :type String) (HeightMapPath :type String) (Hight%20Map%20Strength :type Float%20%28double-precision%29))
  (Variables|Default|SetHight%20Map%20Strength Hight%20Map%20Strength)
  (bind _returnvalue (Class|RuntimeTerrainActor|LoadTexturefromDisk SurfaceMapPath))
  (Variables|Default|SetSurfaceTexture _returnvalue)
  (bind _returnvalue_2 (Class|RuntimeTerrainActor|LoadTexturefromDisk HeightMapPath))
  (Variables|Default|SetHeightmapTexture _returnvalue_2)
  (Utilities|IsValid (Variables|Default|GetSurfaceTexture)
    (:Is%20Valid
      (Utilities|IsValid (Variables|Default|GetHeightmapTexture)
        (:Is%20Valid
          (Default|SetStatus (Variables|Default|GetWidget%20Ref) "Please be patient, this may take some time." "(R=0.000000,G=0.000000,B=0.000000,A=1.000000)")
          (Default|SetProgressBarVisibility (Variables|Default|GetWidget%20Ref) "Visible")
          (Utilities|FlowControl|Delay 1.0)
          (EventDispatchers|BindEventtoOnTerrainGenerationComplete (delegate Custom|OnTerrainGenerationComplete_Event))
          (Class|RuntimeTerrainActor|StartChunkedTerrainGeneration (Variables|Default|GetHight%20Map%20Strength)))
        (:Is%20Not%20Valid
          (Default|SetStatus (Variables|Default|GetWidget%20Ref) "Height Map Path is not valid" "(R=1.000000,G=0.000000,B=0.066323,A=1.000000)"))))
    (:Is%20Not%20Valid
      (Default|SetStatus (Variables|Default|GetWidget%20Ref) "Surface Map Path is not valid" "(R=1.000000,G=0.000000,B=0.066323,A=1.000000)"))))

(event Custom|OnTerrainGenerationComplete_Event
  (Default|SetProgressBarVisibility (Variables|Default|GetWidget%20Ref) "Collapsed"))

(event EventBeginPlay
  (bind _returnvalue (Game|GetPlayerController 0))
  (bind _returnvalue_2 (UserInterface|CreateWidget "/Game/Blueprint/WBP_GenrateTerrainMenu.WBP_GenrateTerrainMenu_C"))
  (bind _output_get (Variables|Default|SetWidget%20Ref _returnvalue_2))
  (EventDispatchers|AssignOnGenrate _output_get (delegate Custom|On%20Genrate_Event))
  (UserInterface|Viewport|AddtoViewport (Variables|Default|GetWidget%20Ref) 0)
  (Variables|/Script/Engine.PlayerController|SetbShowMouseCursor _returnvalue true)
  (Input|SetInputModeGameandUI _returnvalue 0 "DoNotLock" true false))

(fn ConstructionScript)